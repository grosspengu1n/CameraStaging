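; A trigger-volume actor in the Ancient Temple Ruins set that sets off physics props and effects when the player character enters its Box.
; On overlap by bp_ThirdPersonCharacter_SF, it enables physics simulation on every actor in its StaticMeshes array and activates each particle system in its Particles array.
; It then disables the Box's collision so the event fires only once.
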(event `self.Box.OnComponentBeginOverlap`
  (params (OverlappedComponent :type "PrimitiveComponent Object Reference") (OtherActor :type "Actor Object Reference") (OtherComp :type "PrimitiveComponent Object Reference") (OtherBodyIndex :type Integer) (bFromSweep :type Boolean) (SweepResult :type "HitResult Structure (by ref)"))
  (cast `/Game/AncientTempleRuins/Demo/EpicContent/ThirdPersonBP/Blueprints/bp_ThirdPersonCharacter_SF` OtherActor)
  (`|ExecutionSequence`
    (:`then_0`
      (for _array_element (`self.StaticMeshes`)
        (`PrimitiveComponent.SetSimulatePhysics` (`StaticMeshActor.StaticMeshComponent` _array_element) true)))
    (:`then_1`
      (for _array_element_2 (`self.Particles`)
        (`ActorComponent.Activate` (`Emitter.ParticleSystemComponent` _array_element_2) false)))
    (:`then_2`
      (`PrimitiveComponent.SetCollisionEnabled` (`self.Box`) "NoCollision"))))

(fn `UserConstructionScript`)